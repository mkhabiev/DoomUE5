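; Base enemy for a first-person game, drawn as a directional Paper2D flipbook sprite in a 3D world.
; Each tick it derives its state, turns toward a seen player, and picks flipbook and rotation from facing angle and a side test.
; Pawn sensing and damage set the CanSeePlayer blackboard key.
; It provides projectile and line-trace melee attacks, and death stops AI logic, plays death flipbooks and destroys the actor.
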(event `self.ReceiveTick`
  (params (DeltaSeconds :type "Float (single-precision)"))
  (bind _returnvalue (`self.K2_GetActorLocation`))
  (if (> (`KismetMathLibrary.VSize` (`MovementComponent.Velocity` (`self.CharacterMovement`))) 0.0)
    (if (`self.IsAttacking`)
      (switch `/Game/Enemies/AttackState` (`self.AttackState`)
        (:`NewEnumerator0`
          (set `self.EnemyState` "NewEnumerator2"))
        (:`NewEnumerator1`
          (set `self.EnemyState` "NewEnumerator3")))
      (else
        (set `self.EnemyState` "NewEnumerator1")))
    (elif (`self.IsAttacking`)
      (switch `/Game/Enemies/AttackState` (`self.AttackState`)
        (:`NewEnumerator0`
          (set `self.EnemyState` "NewEnumerator2"))
        (:`NewEnumerator1`
          (set `self.EnemyState` "NewEnumerator3")))
      (else
        (set `self.EnemyState` "NewEnumerator0"))))
  (if (`self.IsDead`)
    (`self.HandleDeath`)
    (else
      (if (`self.CanSeePlayer`)
        (`self.RotateTowardsPlayer`))
      (set `self.Degrees` (`KismetMathLibrary.DegAcos` (`KismetMathLibrary.Dot_VectorVector` (`self.GetActorForwardVector`) (`KismetMathLibrary.Normal` (- (`self.K2_GetActorLocation` (`GameplayStatics.GetPlayerCharacter` 0)) _returnvalue)))))
      (if (< (`KismetMathLibrary.Dot_VectorVector` (`self.GetActorRightVector`) _returnvalue) 0.0)
        (`/Engine/EditorBlueprintResources/StandardMacros.CompareFloat` (`self.Degrees`) 180.0
          (:`>`
            (`SceneComponent.K2_SetRelativeRotation` (`self.Paper Flipbook`) (struct :`Yaw` -90.0) false false :!label _label)
            (`PaperFlipbookComponent.SetFlipbook` (`self.Paper Flipbook`) (`|GetArrayItem` (select `/Game/Enemies/EnemyState` (`self.EnemyState`) :`NewEnumerator0` (`self.FlipbooksIDLE`) :`NewEnumerator1` (`self.FlipbooksMoving`) :`NewEnumerator2` (`self.FlipbooksMeleeAttack`) :`NewEnumerator3` (`self.FlipbooksRangeAttack`)))))
          (:`==`
            (goto _label))
          (:`<`
            (`/Engine/EditorBlueprintResources/StandardMacros.CompareFloat` (`self.Degrees`) 135.0
              (:`>`
                (`SceneComponent.K2_SetRelativeRotation` (`self.Paper Flipbook`) (struct :`Yaw` 135.0) false false :!label _label_2)
                (`PaperFlipbookComponent.SetFlipbook` (`self.Paper Flipbook`) (`|GetArrayItem` (select `/Game/Enemies/EnemyState` (`self.EnemyState`) :`NewEnumerator0` (`self.FlipbooksIDLE`) :`NewEnumerator1` (`self.FlipbooksMoving`) :`NewEnumerator2` (`self.FlipbooksMeleeAttack`) :`NewEnumerator3` (`self.FlipbooksRangeAttack`)) 3)))
              (:`==`
                (goto _label_2))
              (:`<`
                (`/Engine/EditorBlueprintResources/StandardMacros.CompareFloat` (`self.Degrees`) 90.0
                  (:`>`
                    (`SceneComponent.K2_SetRelativeRotation` (`self.Paper Flipbook`) (struct :`Yaw` 180.0) false false :!label _label_3)
                    (`PaperFlipbookComponent.SetFlipbook` (`self.Paper Flipbook`) (`|GetArrayItem` (select `/Game/Enemies/EnemyState` (`self.EnemyState`) :`NewEnumerator0` (`self.FlipbooksIDLE`) :`NewEnumerator1` (`self.FlipbooksMoving`) :`NewEnumerator2` (`self.FlipbooksMeleeAttack`) :`NewEnumerator3` (`self.FlipbooksRangeAttack`)) 2)))
                  (:`==`
                    (goto _label_3))
                  (:`<`
                    (`/Engine/EditorBlueprintResources/StandardMacros.CompareFloat` (`self.Degrees`) 45.0
                      (:`>`
                        _)
                      (:`==`
                        _)
                      (:`<`
                        (goto _label)))
                    (`SceneComponent.K2_SetRelativeRotation` (`self.Paper Flipbook`) (struct :`Yaw` 45.0) false false)
                    (`PaperFlipbookComponent.SetFlipbook` (`self.Paper Flipbook`) (`|GetArrayItem` (select `/Game/Enemies/EnemyState` (`self.EnemyState`) :`NewEnumerator0` (`self.FlipbooksIDLE`) :`NewEnumerator1` (`self.FlipbooksMoving`) :`NewEnumerator2` (`self.FlipbooksMeleeAttack`) :`NewEnumerator3` (`self.FlipbooksRangeAttack`)) 1))))))))
        (else
          (`/Engine/EditorBlueprintResources/StandardMacros.CompareFloat` (`self.Degrees`) 180.0
            (:`>`
              (`SceneComponent.K2_SetRelativeRotation` (`self.Paper Flipbook`) (struct :`Yaw` -45.0) false false :!label _label_4)
              (`PaperFlipbookComponent.SetFlipbook` (`self.Paper Flipbook`) (`|GetArrayItem` (select `/Game/Enemies/EnemyState` (`self.EnemyState`) :`NewEnumerator0` (`self.FlipbooksIDLE`) :`NewEnumerator1` (`self.FlipbooksMoving`) :`NewEnumerator2` (`self.FlipbooksMeleeAttack`) :`NewEnumerator3` (`self.FlipbooksRangeAttack`)) 1)))
            (:`==`
              (goto _label_4))
            (:`<`
              (`/Engine/EditorBlueprintResources/StandardMacros.CompareFloat` (`self.Degrees`) 135.0
                (:`>`
                  (`SceneComponent.K2_SetRelativeRotation` (`self.Paper Flipbook`) (struct :`Yaw` 90.0) false false :!label _label_5)
                  (`PaperFlipbookComponent.SetFlipbook` (`self.Paper Flipbook`) (`|GetArrayItem` (select `/Game/Enemies/EnemyState` (`self.EnemyState`) :`NewEnumerator0` (`self.FlipbooksIDLE`) :`NewEnumerator1` (`self.FlipbooksMoving`) :`NewEnumerator2` (`self.FlipbooksMeleeAttack`) :`NewEnumerator3` (`self.FlipbooksRangeAttack`)) 4)))
                (:`==`
                  (goto _label_5))
                (:`<`
                  (`/Engine/EditorBlueprintResources/StandardMacros.CompareFloat` (`self.Degrees`) 90.0
                    (:`>`
                      (`SceneComponent.K2_SetRelativeRotation` (`self.Paper Flipbook`) (struct :`Yaw` 45.0) false false :!label _label_6)
                      (`PaperFlipbookComponent.SetFlipbook` (`self.Paper Flipbook`) (`|GetArrayItem` (select `/Game/Enemies/EnemyState` (`self.EnemyState`) :`NewEnumerator0` (`self.FlipbooksIDLE`) :`NewEnumerator1` (`self.FlipbooksMoving`) :`NewEnumerator2` (`self.FlipbooksMeleeAttack`) :`NewEnumerator3` (`self.FlipbooksRangeAttack`)) 5)))
                    (:`==`
                      (goto _label_6))
                    (:`<`
                      (`/Engine/EditorBlueprintResources/StandardMacros.CompareFloat` (`self.Degrees`) 45.0
                        (:`>`
                          _)
                        (:`==`
                          _)
                        (:`<`
                          _))
                      (`SceneComponent.K2_SetRelativeRotation` (`self.Paper Flipbook`) (struct :`Yaw` -45.0) false false)
                      (`PaperFlipbookComponent.SetFlipbook` (`self.Paper Flipbook`) (`|GetArrayItem` (select `/Game/Enemies/EnemyState` (`self.EnemyState`) :`NewEnumerator0` (`self.FlipbooksIDLE`) :`NewEnumerator1` (`self.FlipbooksMoving`) :`NewEnumerator2` (`self.FlipbooksMeleeAttack`) :`NewEnumerator3` (`self.FlipbooksRangeAttack`)) 6)))))))))))))

(event `RotateTowardsPlayer`
  ;[0.05521 0.05521 0.05521] Handle enemy rotation
  (`self.K2_SetActorRotation` (`KismetMathLibrary.RInterpTo` (`self.K2_GetActorRotation`) (`KismetMathLibrary.FindLookAtRotation` (`self.K2_GetActorLocation`) (`self.K2_GetActorLocation` (`GameplayStatics.GetPlayerCharacter` 0))) (`GameplayStatics.GetWorldDeltaSeconds`) (`self.RotationSpeed`))))

(event `self.PawnSensing.OnSeePawn`
  (params (Pawn :type "Pawn Object Reference"))
  ;[0.1219 0.1219 0.1219] Handle enemy vision
  (cast `/Game/FirstPerson/Blueprints/BP_FirstPersonCharacter` Pawn)
  (set `self.CanSeePlayer` true)
  (`BlackboardComponent.SetValueAsBool` (`AIBlueprintHelperLibrary.GetBlackboard` null) "CanSeePlayer" true)
  (`KismetSystemLibrary.RetriggerableDelay` 0.7)
  (set `self.CanSeePlayer` false)
  (`BlackboardComponent.SetValueAsBool` (`AIBlueprintHelperLibrary.GetBlackboard` null) "CanSeePlayer" false))

(event `SpawnProjectile`
  ;[0.06771 0.06771 0.06771] Attack system
  ;;[1 1 1] Range attck
  (set `self.IsAttacking` true)
  (set `self.AttackState` "NewEnumerator1")
  (`MovementComponent.StopMovementImmediately` (`self.CharacterMovement`))
  (`|SpawnActorFromClass` (`self.EnemyProjectile`) (`SceneComponent.K2_GetComponentToWorld` (`self.ProjectileSpawn`)) "Undefined" "MultiplyWithRoot" null (`self.ProjectileSpeed`) (`self.ProjectileDamage`) null)
  (`KismetSystemLibrary.RetriggerableDelay` (+ (`self.FireRate`) 0.1))
  (set `self.IsAttacking` false))

(event `MeleeAttack`
  (bind _returnvalue (`self.K2_GetActorLocation`))
  ;[0.06771 0.06771 0.06771] Attack system
  ;;[0.9991 0.999 1] Melee attack
  (set `self.IsAttacking` true)
  (set `self.AttackState` "NewEnumerator0")
  (bind _outhit (`KismetSystemLibrary.LineTraceSingleForObjects` _returnvalue (+ _returnvalue (* (`self.GetActorForwardVector`) 150.0)) (`|MakeArray` "ObjectTypeQuery3" :!type "EObjectTypeQuery Enum") false (`|MakeArray` self :!type "Actor Object Reference") "ForDuration"))
  (bind (_bblockinghit _binitialoverlap _time _distance _location _impactpoint _normal _impactnormal _physmat _hitactor) (`GameplayStatics.BreakHitResult` _outhit))
  (if (== _hitactor (`GameplayStatics.GetPlayerCharacter` 0))
    (`GameplayStatics.ApplyDamage` _hitactor (`self.EnemyDamage`)))
  (`KismetSystemLibrary.RetriggerableDelay` (+ (`self.MeleeRate`) 0.1))
  (set `self.IsAttacking` false))

(event `self.ReceiveAnyDamage`
  (params (Damage :type "Float (single-precision)") (DamageType :type "DamageType Object Reference") (InstigatedBy :type "Controller Object Reference") (DamageCauser :type "Actor Object Reference"))
  ;[1 1 1] Enemy damage
  (bind _output_get (set `self.Health` (- (`self.Health`) Damage)))
  (if (<= _output_get 0.0)
    (set `self.IsDead` true)
    (else
      (set `self.CanSeePlayer` true)
      (`BlackboardComponent.SetValueAsBool` (`AIBlueprintHelperLibrary.GetBlackboard` null) "CanSeePlayer" true))))

(event `HandleDeath`
  (bind _paper_flipbook (`self.Paper Flipbook`))
  (bind (_returnvalue_roll _returnvalue_pitch _returnvalue_yaw) (`KismetMathLibrary.BreakRotator` (`KismetMathLibrary.FindLookAtRotation` (`self.K2_GetActorLocation`) (`self.K2_GetActorLocation` (`GameplayStatics.GetPlayerCharacter` 0)))))
  ;[1 1 1] Enemy Death System
  (`self.K2_SetActorRotation` (`KismetMathLibrary.MakeRotator` 0.0 0.0 _returnvalue_yaw))
  (`/Engine/EditorBlueprintResources/StandardMacros.DoOnce` false
    (:`Completed`
      (`BrainComponent.StopLogic` (`AIController.BrainComponent` (`AIBlueprintHelperLibrary.GetAIController` self)) "IsDead")
      (`CharacterMovementComponent.SetMovementMode` (`self.CharacterMovement`) "MOVE_Flying" 0)
      (`PrimitiveComponent.SetCollisionEnabled` (`self.CapsuleComponent`) "NoCollision")
      (`ActorComponent.Deactivate` (`self.CharacterMovement`))
      (`SceneComponent.K2_SetRelativeRotation` _paper_flipbook (struct :`Yaw` -90.0) false false)
      (`PaperFlipbookComponent.SetFlipbook` _paper_flipbook (`self.EnemyDeathFlipbook`))
      (`KismetSystemLibrary.Delay` (- (`PaperFlipbookComponent.GetFlipbookLength` (`self.Paper Flipbook`)) 0.2))
      (`self.K2_AddActorLocalOffset` (0.0 0.0 -45.0))
      (`PaperFlipbookComponent.SetFlipbook` (`self.Paper Flipbook`) (`self.EnemyDeadbodyFlipbook`))
      (`KismetSystemLibrary.Delay` 4.0)
      (`self.K2_DestroyActor`))))

(fn `UserConstructionScript`)