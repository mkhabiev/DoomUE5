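; BP_BaseWeapon is the base weapon Blueprint, providing shared firing, ammo and sound logic, with empty ShootWeapon and StopShooting events.
; FireWeapon does a debug-drawn line trace hitscan that applies damage and spawns blood on Enemy-tagged actors, while FireProjectile spawns a projectile with speed and damage.
; EnoughAmmo and DecreaseAmmo switch on AmmoType, using ammo counts stored on the cached first-person character and updating its HUD.
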(event `self.ReceiveBeginPlay`
  (bind _asbp_first_person_character (cast `/Game/FirstPerson/Blueprints/BP_FirstPersonCharacter` (`GameplayStatics.GetPlayerCharacter` 0)))
  (set `self.PlayerCharacterRef` _asbp_first_person_character))

(event `ShootWeapon`)

(event `StopShooting`)

(event `DecreaseAmmo`
  (bind _playercharacterref (`self.PlayerCharacterRef`))
  (bind _playercharacterref_2 (`self.PlayerCharacterRef`))
  (bind _playercharacterref_3 (`self.PlayerCharacterRef`))
  (bind _playercharacterref_4 (`self.PlayerCharacterRef`))
  (switch `/Game/Blueprints/Weapons/Ammo` (`self.AmmoType`)
    (:`NewEnumerator0`
      (`/Engine/EditorBlueprintResources/StandardMacros.DecrementInt` (`/Game/FirstPerson/Blueprints/BP_FirstPersonCharacter.Bullet` _playercharacterref_2)
        (:`  `
          (`/Game/Blueprints/UI/PlayerHUD.UpdateBulletAmmo` (`/Game/FirstPerson/Blueprints/BP_FirstPersonCharacter.PlayerHUD` _playercharacterref_2)))))
    (:`NewEnumerator1`
      (`/Engine/EditorBlueprintResources/StandardMacros.DecrementInt` (`/Game/FirstPerson/Blueprints/BP_FirstPersonCharacter.Shell` _playercharacterref_3)
        (:`  `
          (`/Game/Blueprints/UI/PlayerHUD.UpdateShellAmmo` (`/Game/FirstPerson/Blueprints/BP_FirstPersonCharacter.PlayerHUD` _playercharacterref_3)))))
    (:`NewEnumerator2`
      (`/Engine/EditorBlueprintResources/StandardMacros.DecrementInt` (`/Game/FirstPerson/Blueprints/BP_FirstPersonCharacter.Rocket` _playercharacterref_4)
        (:`  `
          (`/Game/Blueprints/UI/PlayerHUD.UpdateRocketAmmo` (`/Game/FirstPerson/Blueprints/BP_FirstPersonCharacter.PlayerHUD` _playercharacterref_4)))))
    (:`NewEnumerator3`
      (`/Engine/EditorBlueprintResources/StandardMacros.DecrementInt` (`/Game/FirstPerson/Blueprints/BP_FirstPersonCharacter.Cell` _playercharacterref)
        (:`  `
          (`/Game/Blueprints/UI/PlayerHUD.UpdateCellAmmo` (`/Game/FirstPerson/Blueprints/BP_FirstPersonCharacter.PlayerHUD` _playercharacterref)))))))

(event `PlayWeaponSound`
  (`GameplayStatics.PlaySoundAtLocation` (`self.Sound`) (`self.K2_GetActorLocation`) (struct) 1.0 1.0 0.0 null null null null))

(fn `EnoughAmmo`
  (returns (HasAmmo :type Boolean))
  (switch `/Game/Blueprints/Weapons/Ammo` (`self.AmmoType`)
    (:`NewEnumerator0`
      (if (> (`/Game/FirstPerson/Blueprints/BP_FirstPersonCharacter.Bullet` (`self.PlayerCharacterRef`)) 0)
        (return true)
        (else
          (return false))))
    (:`NewEnumerator1`
      (if (> (`/Game/FirstPerson/Blueprints/BP_FirstPersonCharacter.Shell` (`self.PlayerCharacterRef`)) 0)
        (return true)
        (else
          (return false))))
    (:`NewEnumerator2`
      (if (> (`/Game/FirstPerson/Blueprints/BP_FirstPersonCharacter.Rocket` (`self.PlayerCharacterRef`)) 0)
        (return true)
        (else
          (return false))))
    (:`NewEnumerator3`
      (if (> (`/Game/FirstPerson/Blueprints/BP_FirstPersonCharacter.Cell` (`self.PlayerCharacterRef`)) 0)
        (return true)
        (else
          (return false))))))

(fn `FireProjectile`
  (`|SpawnActorFromClass` (`self.Projectile`) (`SceneComponent.K2_GetComponentToWorld` (`self.ProjectileTransform`)) "Undefined" "MultiplyWithRoot" null (`self.ProjectileSpeed`) (`self.WeaponDamage`) null))

(fn `FireWeapon`
  (bind _returnvalue (`SceneComponent.K2_GetComponentLocation` (`self.LineTrace`)))
  (bind (_outhit _returnvalue_2) (`KismetSystemLibrary.LineTraceSingleForObjects` _returnvalue (+ _returnvalue (* (`KismetMathLibrary.GetForwardVector` (`SceneComponent.K2_GetComponentRotation` (`self.LineTrace`))) (`self.LinetraceDistance`))) (`|MakeArray` "ObjectTypeQuery1" "ObjectTypeQuery2" "ObjectTypeQuery3" :!type "EObjectTypeQuery Enum") false (`|MakeArray` self (`GameplayStatics.GetPlayerCharacter` 0) :!type "Actor Object Reference") "ForDuration"))
  (if _returnvalue_2
    (bind (_bblockinghit _binitialoverlap _time _distance _location _impactpoint _normal _impactnormal _physmat _hitactor) (`GameplayStatics.BreakHitResult` _outhit))
    (`GameplayStatics.ApplyDamage` _hitactor (`self.WeaponDamage`))
    (if (`self.ActorHasTag` _hitactor "Enemy")
      (`|SpawnActorFromClass` "/Game/Enemies/Blood/BP_Blood.BP_Blood_C" (`KismetMathLibrary.MakeTransform` _location) "Undefined" "MultiplyWithRoot" null null))))

(fn `UserConstructionScript`)